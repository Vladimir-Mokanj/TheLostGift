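; Main menu game mode that opens the game's front-end screens: main menu, singleplayer, multiplayer and settings.
; Each show event lazily creates its widget, caches it for reuse and adds it to the viewport.
; Showing the main menu also enables the mouse cursor, and a separate event quits the game.
; Nothing here removes widgets or calls these events itself.
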(event `ShowMainMenu`
  ;[1 1 1 1 30] MainMenu Events
  ;;[1 1 1] Display Main Menu to the screen / Make mouse visible
  (`/Engine/EditorBlueprintResources/StandardMacros.IsValid` (`self.MainMenuWB`)
    (:`Is Valid`
      _)
    (:`Is Not Valid`
      (bind _returnvalue (`|CreateWidget` "/Game/_Production/Blueprints/UI/MainMenu/MainMenu_WB.MainMenu_WB_C"))
      (set `self.MainMenuWB` _returnvalue)))
  (`UserWidget.AddToViewport` (`self.MainMenuWB`) 0)
  (set `PlayerController.bShowMouseCursor` true (`GameplayStatics.GetPlayerController` 0)))

(event `ShowSingleplayer`
  ;[1 1 1 1 30] MainMenu Events
  ;;[1 1 1] Display Singleplayer to the screen
  (`/Engine/EditorBlueprintResources/StandardMacros.IsValid` (`self.SingleplayerWB`)
    (:`Is Valid`
      _)
    (:`Is Not Valid`
      (bind _returnvalue (`|CreateWidget` "/Game/_Production/Blueprints/UI/MainMenu/Singleplayer_WB.Singleplayer_WB_C"))
      (set `self.SingleplayerWB` _returnvalue)))
  (`UserWidget.AddToViewport` (`self.SingleplayerWB`) 0))

(event `ShowMultiplayer`
  ;[1 1 1 1 30] MainMenu Events
  ;;[1 1 1] Display Multiplayer to the screen
  (`/Engine/EditorBlueprintResources/StandardMacros.IsValid` (`self.MultiplayerWB`)
    (:`Is Valid`
      _)
    (:`Is Not Valid`
      (bind _returnvalue (`|CreateWidget` "/Game/_Production/Blueprints/UI/MainMenu/Multiplayer_WB.Multiplayer_WB_C"))
      (set `self.MultiplayerWB` _returnvalue)))
  (`UserWidget.AddToViewport` (`self.MultiplayerWB`) 0))

(event `ShowSettings`
  ;[1 1 1 1 30] MainMenu Events
  ;;[1 1 1] Display Settings to the screen
  (`/Engine/EditorBlueprintResources/StandardMacros.IsValid` (`self.SettingsWB`)
    (:`Is Valid`
      _)
    (:`Is Not Valid`
      (bind _returnvalue (`|CreateWidget` "/Game/_Production/Blueprints/UI/MainMenu/Settings_WB.Settings_WB_C"))
      (set `self.SettingsWB` _returnvalue)))
  (`UserWidget.AddToViewport` (`self.SettingsWB`) 0))

(event `QuitGame`
  ;[1 1 1 1 30] MainMenu Events
  ;;[1 1 1] Quit the Game
  (`KismetSystemLibrary.QuitGame` null "Quit"))

(fn `UserConstructionScript`)